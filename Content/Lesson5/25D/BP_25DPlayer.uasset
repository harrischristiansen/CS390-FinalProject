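; BP_25DPlayer is the player pawn for a 2.5D level, with jumping, world-axis movement and an optional auto-run along Y.
; On begin play it detaches the camera root and stores the start location, so each tick the camera follows the player only along Y.
; Tick also applies auto-move, which disables manual right input, reloads the "25D" level when the player falls below zero height, and updates a text timer from game time.
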(event EventBeginPlay
  ;[1 1 1] Prep Camera
  (Variables|/Script/Engine.CameraComponent|SetbUsePawnControlRotation (Variables|Default|GetCamera) (Class|HeadMountedDisplayFunctionLibrary|IsHeadMountedDisplayEnabled))
  (Class|SceneComponent|DetachfromParent (Variables|Default|GetCameraRoot) true true)
  (Variables|Default|SetCameraStartLocation (Transformation|GetActorLocation)))

(event EventTick
  (params (DeltaSeconds :type Float%20%28single-precision%29))
  (bind _camerastartlocation (Variables|Default|GetCameraStartLocation))
  ;[1 1 1] Move Camera
  (Transformation|SetWorldLocation (Variables|Default|GetCameraRoot) (Math|Vector|MakeVector (.x _camerastartlocation) (.y (Transformation|GetActorLocation)) (.z _camerastartlocation)) false false)
  (Utilities|FlowControl|Sequence
    (:then_0
      ;[1 1 1] AutoMove
      (if (Variables|Default|GetAutoMove)
        (Pawn|Input|AddMovementInput "0,1.000000, 0" 1.0 false)))
    (:then_1
      ;[1 1 1] Respawn When Fall
      (if (< (.z (Transformation|GetActorLocation)) 0.0)
        (Game|OpenLevel(byName) "25D")))
    (:then_2
      ;[1 1 1] Update Timer Text
      (Rendering|Components|TextRender|SetText (Variables|Default|GetTextRender) (Utilities|Text|ToText(String) (Utilities|String|BuildString(Integer) "" "Time: " (Math|Float|Round (Utilities|Time|GetGameTimeinSeconds))))))))

(event Input|ActionEvents|InputActionJump
  (params (Key :type Key%20Structure :default "AnyKey"))
  ;[1 1 1] Movement
  (:Pressed
    (Character|Jump))
  (:Released
    (Character|StopJumping)))

(event Input|AxisEvents|InputAxisMoveRight
  (params (AxisValue :type Float%20%28single-precision%29))
  ;[1 1 1] Movement
  (if (not (Variables|Default|GetAutoMove))
    (Pawn|Input|AddMovementInput "0,1.000000, 0" AxisValue false)))

(event Input|AxisEvents|InputAxisMoveForward
  (params (AxisValue :type Float%20%28single-precision%29))
  ;[1 1 1] Movement
  (Pawn|Input|AddMovementInput "1.000000, 0, 0" AxisValue false))

(fn ConstructionScript)