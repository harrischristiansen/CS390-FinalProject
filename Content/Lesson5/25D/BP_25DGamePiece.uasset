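; BP_25DGamePiece is the playable piece of a 2.5D lesson game, supporting jump input.
; On BeginPlay it registers itself as GamePieceActor on the player pawn, a BP_25DFirstPerson camera, then sets AutoMove after a short delay.
; Auto-run, axis movement and reload-level-on-fall logic exist but are disconnected, so the movement axis events do nothing and AutoMove has no effect here.
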(event EventBeginPlay
  (Utilities|FlowControl|Sequence
    (:then_0
      ;[1 1 1] Identify Self To Camera
      (bind _asbp_25dfirst_person (Utilities|Casting|CastToBP_25DFirstPerson (Game|Player|GetPlayerPawn 0)))
      (Variables|/Game/Lesson5/25D/BP_25DFirstPerson.BP_25DFirstPerson_C|SetgamePieceActor _asbp_25dfirst_person self))
    (:then_1
      ;[1 1 1] Start Game
      (Utilities|FlowControl|Delay 2.0)
      (Variables|Default|SetAutoMove true))))

(event Input|ActionEvents|InputActionJump
  (params (Key :type Key%20Structure :default "AnyKey"))
  ;[1 1 1] Movement
  (:Pressed
    (Character|Jump))
  (:Released
    (Character|StopJumping)))

(event Input|AxisEvents|InputAxisMoveRight
  (params (AxisValue :type Float%20%28single-precision%29))
  ;[1 1 1] Movement
)

(event Input|AxisEvents|InputAxisMoveForward
  (params (AxisValue :type Float%20%28single-precision%29))
  ;[1 1 1] Movement
)

(fn ConstructionScript)