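; 2.5D camera actor, named as not used, that becomes the player's view target on BeginPlay and fades in from black.
; Each tick it follows the pawn along Y at fixed X and height, applies an HMD transform in VR, and updates an elapsed-time text.
; Fades use timelines driving Opacity on the BlindingBox's dynamic material; FadeToBlack is not called here.
; Aim-at-player rotation logic is disconnected.
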(event Custom|FadeFromBlack
  ;[1 1 1] Fade from Black
  (bind _returnvalue (Rendering|Material|CreateDynamicMaterialInstance (Variables|Default|GetBlindingBox) 0 "/Game/Materials/UI/M_Fade.M_Fade" :!class /Script/Engine.PrimitiveComponent))
  (Variables|Default|SetFadeDMI _returnvalue)
  (bind _data (Timeline|FadeIn PlayFromStart)
    (:Update
      (Rendering|Material|SetScalarParameterValue (Variables|Default|GetFadeDMI) "Opacity" _data :!class /Script/Engine.MaterialInstanceDynamic))))

(event Custom|FadeToBlack
  ;[1 1 1] Fade to Black
  (bind _returnvalue (Rendering|Material|CreateDynamicMaterialInstance (Variables|Default|GetBlindingBox) 0 "/Game/Materials/UI/M_Fade.M_Fade" :!class /Script/Engine.PrimitiveComponent))
  (Variables|Default|SetFadeDMI _returnvalue)
  (bind _data (Timeline|FadeOut PlayFromStart)
    (:Update
      (Rendering|Material|SetScalarParameterValue (Variables|Default|GetFadeDMI) "Opacity" _data :!class /Script/Engine.MaterialInstanceDynamic))))

(event EventTick
  (params (DeltaSeconds :type Float%20%28single-precision%29))
  (Utilities|FlowControl|Sequence
    (:then_0
      ;[1 1 1] Follow Player Location
      (Transformation|SetActorLocation (Math|Vector|MakeVector 0.0 (.y (Transformation|GetActorLocation (Game|Player|GetPlayerPawn 0))) 4e+03) false false))
    (:then_1
      (if (Class|HeadMountedDisplayFunctionLibrary|IsHeadMountedDisplayEnabled)
        ;[1 1 1] VR Control Rotation
        (bind _newtransform (CallFunction|TransformwithHMD))
        (Transformation|SetActorLocationAndRotation (.location _newtransform) (.rotation _newtransform))))
    (:then_2
      ;[1 1 1] Timer
      (Rendering|Components|TextRender|SetText (Variables|Default|GetTextRender) (Utilities|Text|ToText(String) (Utilities|String|BuildString(Integer) "" "Time: " (Math|Float|Round (Utilities|Time|GetGameTimeinSeconds))))))))

(event EventBeginPlay
  ;[1 1 1] Activate Camera
  (Game|Player|SetViewTargetwithBlend (Game|GetPlayerController 0) self 0.0 "VTBlend_Linear" 0.0 false)
  (CallFunction|FadefromBlack))

(fn ConstructionScript
  (bind _returnvalue (Rendering|Material|CreateDynamicMaterialInstance (Variables|Default|GetBlindingBox) 0 0 :!class /Script/Engine.PrimitiveComponent))
  (Variables|Default|SetFadeDMI _returnvalue))