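; BP_Segment1 is a floor segment for a 2.5D game that chains into an endless track.
; When a BP_25DGamePiece overlaps its trigger, it asks 25DGameMode to add a floor tile, then destroys itself after a delay.
; GetAttachTransform exposes the AttachPoint world transform, presumably for placing the next segment.
; The trigger also writes the player's CurrentMoveSpeed back unchanged, so speed is unaffected.
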(event OnComponentBeginOverlap(TriggerAddFloorTile)
  (params (OtherActor :type Actor%20Object%20Reference) (OtherComp :type Primitive%20Component%20Object%20Reference) (OtherBodyIndex :type Integer) (bFromSweep :type Boolean) (SweepResult :type Hit%20Result%20Structure%20%28by%20ref%29))
  ;[1 1 1] Add New Obstacles Segment
  (Utilities|Casting|CastToBP_25DGamePiece OtherActor)
  (bind _as25dgame_mode (Utilities|Casting|CastTo25DGameMode (Game|GetGameMode)))
  (Default|AddFloorTile _as25dgame_mode)
  (bind _asbp_25dfirst_person (Utilities|Casting|CastToBP_25DFirstPerson (Game|Player|GetPlayerPawn 0)))
  (Variables|/Game/Lesson5/25D/BP_25DFirstPerson.BP_25DFirstPerson_C|SetcurrentMoveSpeed _asbp_25dfirst_person (Variables|/Game/Lesson5/25D/BP_25DFirstPerson.BP_25DFirstPerson_C|GetcurrentMoveSpeed _asbp_25dfirst_person))
  ;[1 1 1] Destroy Self
  (Utilities|FlowControl|Delay 3e+01)
  (Actor|DestroyActor))

(fn ConstructionScript)

(fn GetAttachTransform
  (return (Transformation|GetWorldTransform (Variables|Default|GetAttachPoint))))